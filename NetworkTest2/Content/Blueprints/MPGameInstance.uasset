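; MPGameInstance is a multiplayer game instance Blueprint that wraps LAN session management in four events: host, search, join and destroy.
; Each event runs an async session node on player controller 0, mostly printing the outcome on screen.
; Search stores found sessions in SessionResults, and join always takes the first entry without a bounds check.
; Hosting sets zero public connections and triggers no map travel.
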(event Custom|Search%20Game
  ;[1 1 1] Search Games
  (bind _results (|FindSessions (Game|GetPlayerController 0) 10 true)
    (:OnSuccess
      (Variables|Default|SetSessionResults _results))
    (:OnFailure
      (Development|PrintString "No Sessions found!"))))

(event Custom|Destroy%20Game
  ;[1 1 1] Destroy Game
  (|DestroySession (Game|GetPlayerController 0)
    (:OnSuccess
      (Development|PrintString "Succesfully destroyed session!"))
    (:OnFailure
      (Development|PrintString "Session destroyed faild!"))))

(event Custom|Host%20Game
  ;[1 1 1] Host Game
  (|Session (Game|GetPlayerController 0) 0 true
    (:OnSuccess
      (Development|PrintString "Session created!"))
    (:OnFailure
      (Development|PrintString "Creation failed!"))))

(event Custom|Join%20Game
  ;[1 1 1] Join Game
  (|JoinSession (Game|GetPlayerController 0) (Utilities|Array|Get(acopy) (Variables|Default|GetSessionResults))
    (:OnSuccess
      (Development|PrintString "Succefully joined to session!"))
    (:OnFailure
      (Development|PrintString "Failed to join session!"))))